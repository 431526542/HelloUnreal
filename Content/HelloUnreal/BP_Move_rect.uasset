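; BP_Move_rect is an actor that moves its Cube component around a rectangular loop in the local XZ plane.
; Each Tick switches on the MoveType state (Right, Up, Left, Down) and offsets the cube's relative location by a fixed step without sweep.
; The state advances when the cube reaches EndPoint on the outbound legs or drops below zero on the return legs, so speed depends on frame rate.
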(event EventTick
  (params (DeltaSeconds :type Float%20%28single-precision%29))
  (bind _cube (Variables|Default|GetCube))
  (bind _cube_2 (Variables|Default|GetCube))
  (switch Utilities|FlowControl|Switch|SwitchonEn_movetypr (Variables|Default|GetMoveType)
    (:NewEnumerator0
      (Transformation|AddRelativeLocation _cube_2 "10.000000, 0, 0" false false)
      (if (>= (.x (Variables|/Script/Engine.SceneComponent|GetRelativeLocation _cube_2)) (Variables|Default|GetEndPoint))
        (Variables|Default|SetMoveType "NewEnumerator1")))
    (:NewEnumerator1
      (Transformation|AddRelativeLocation (Variables|Default|GetCube) "0.000000, 0,10.000000" false false)
      (if (>= (.z (Variables|/Script/Engine.SceneComponent|GetRelativeLocation _cube_2)) (Variables|Default|GetEndPoint))
        (Variables|Default|SetMoveType "NewEnumerator2")))
    (:NewEnumerator2
      (Transformation|AddRelativeLocation _cube "-10.000000, 0,0.000000" false false)
      (if (< (.x (Variables|/Script/Engine.SceneComponent|GetRelativeLocation _cube)) 0.0)
        (Variables|Default|SetMoveType "NewEnumerator3")))
    (:NewEnumerator3
      (Transformation|AddRelativeLocation (Variables|Default|GetCube) "0.000000, 0,-10.000000" false false)
      (if (< (.z (Variables|/Script/Engine.SceneComponent|GetRelativeLocation _cube)) 0.0)
        (Variables|Default|SetMoveType "NewEnumerator0")))))

(fn ConstructionScript)