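; Actor Blueprint that slides its Cube component back and forth along the local X axis.
; Each Tick offsets the cube by a fixed step, using the IsMoveRight flag to pick the direction.
; The flag flips when relative X reaches EndPoint or drops below zero.
; The step is per frame and not scaled by delta time, so speed depends on frame rate.
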(event EventTick
  (params (DeltaSeconds :type Float%20%28single-precision%29))
  (bind _cube (Variables|Default|GetCube))
  (if (Variables|Default|GetIsMoveRight)
    (Transformation|AddRelativeLocation _cube "5.000000, 0, 0" false false)
    (if (>= (.x (Variables|/Script/Engine.SceneComponent|GetRelativeLocation _cube)) (Variables|Default|GetEndPoint))
      (Variables|Default|SetIsMoveRight false))
    (else
      (Transformation|AddRelativeLocation (Variables|Default|GetCube) "-5.000000, 0, 0" false false)
      (if (< (.x (Variables|/Script/Engine.SceneComponent|GetRelativeLocation _cube)) 0.0)
        (Variables|Default|SetIsMoveRight true)))))

(fn ConstructionScript)