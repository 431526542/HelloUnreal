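; BP_ㄴMove is a Blueprint that moves its Sphere component back and forth along an L-shaped path in a continuous loop.
; Each Tick switches on the Totla state and adds a fixed relative offset, without sweep or delta-time scaling.
; The sphere travels +X, then +Z until each reaches EndPoint, then retraces both legs until below zero.
; The Left state moves down in Z and Down moves back in X, despite their names.
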(event EventTick
  (params (DeltaSeconds :type Float%20%28single-precision%29))
  (bind _sphere (Variables|Default|GetSphere))
  (bind _sphere_2 (Variables|Default|GetSphere))
  (bind _sphere_3 (Variables|Default|GetSphere))
  (bind _sphere_4 (Variables|Default|GetSphere))
  (switch Utilities|FlowControl|Switch|SwitchonEn_movetypr (Variables|Default|GetTotla)
    (:NewEnumerator0
      (Transformation|AddRelativeLocation _sphere_3 "10.000000, 0, 0" false false)
      (if (>= (.x (Variables|/Script/Engine.SceneComponent|GetRelativeLocation _sphere_3)) (Variables|Default|GetEndPoint))
        (Variables|Default|SetTotla "NewEnumerator1")))
    (:NewEnumerator1
      (Transformation|AddRelativeLocation _sphere_4 "0.000000, 0,10.000000" false false)
      (if (>= (.z (Variables|/Script/Engine.SceneComponent|GetRelativeLocation _sphere_4)) (Variables|Default|GetEndPoint))
        (Variables|Default|SetTotla "NewEnumerator2")))
    (:NewEnumerator2
      (Transformation|AddRelativeLocation _sphere_2 "0.000000, 0,-10.000000" false false)
      (if (< (.z (Variables|/Script/Engine.SceneComponent|GetRelativeLocation _sphere_2)) 0.0)
        (Variables|Default|SetTotla "NewEnumerator3")))
    (:NewEnumerator3
      (Transformation|AddRelativeLocation _sphere "-10.000000, 0,-0.000000" false false)
      (if (< (.x (Variables|/Script/Engine.SceneComponent|GetRelativeLocation _sphere)) 0.0)
        (Variables|Default|SetTotla "NewEnumerator0")))))

(fn ConstructionScript)